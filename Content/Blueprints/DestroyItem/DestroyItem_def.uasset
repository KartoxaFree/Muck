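; Destructible world object that drops an item when its health runs out.
; The construction script sets the cube's mesh from its Description data, and BeginPlay initializes the health component's health and damage values.
; The component's OnDeath event calls Death, which prints a debug string, spawns an Items_Base at the cube's location with the stack amount and nested item description, then destroys the actor.
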(event OnDeath(Health_Component)
  (CallFunction|Death))

(event EventBeginPlay
  (Variables|/Game/Blueprints/Health/Health_Component.Health_Component_C|SetHealth%20Actor (Variables|Default|GetHealth_Component) 1e+02)
  (Variables|/Game/Blueprints/Health/Health_Component.Health_Component_C|SetDamage%20Actor (Variables|Default|GetHealth_Component) 1e+02))

(fn ConstructionScript
  (Components|StaticMesh|SetStaticMesh (Variables|Default|GetCube) (Variables|/Game/Blueprints/DestroyItem/ItemData/DestructbleObject.DestructbleObject_C|GetMesh (Variables|Default|GetDescription))))

(fn Death
  (Development|PrintString "Hello")
  (Game|SpawnActorfromClass "/Game/Blueprints/InteractItem/Items_Base.Items_Base_C" (Math|Transform|MakeTransform (Transformation|GetWorldLocation (Variables|Default|GetCube)) "0, 0, 0" "1.000000,1.000000,1.000000") "Undefined" "MultiplyWithRoot" 0 (Variables|Default|GetAmount) (Variables|/Game/Blueprints/DestroyItem/ItemData/DestructbleObject.DestructbleObject_C|GetDescription (Variables|Default|GetDescription)) 0)
  (Actor|DestroyActor))