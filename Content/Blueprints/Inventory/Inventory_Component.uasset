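; Grid inventory component that stores item stacks in a map keyed by cell position, bounded by InventorySize.
; Items are added and removed one unit at a time up to each stack limit, while drag-drop moves stacks or merges matching ones.
; SpawnItem drops a stack into the world, using forward sphere and downward line traces for placement, then clears its cell.
; Removals and drag-drop changes refresh the Player's inventory widget; adds do not.
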(event EventBeginPlay)

(event EventTick
  (params (DeltaSeconds :type Float%20%28single-precision%29)))

(fn AddItem
  (params (Description :type Item%20Data%20Object%20Reference))
  (bind _inventory_size (Variables|Default|GetInventory%20Size))
  (bind _inventory_size_2 (Variables|Default|GetInventory%20Size))
  (for _index (range 0 (- (.y _inventory_size_2) 1))
    (for _index_2 (range 0 (- (.x _inventory_size_2) 1))
      (if (== Description (.description (.Value (Utilities|Map|Find (Variables|Default|GetStacks) (Utilities|Struct|MakeIntPoint _index_2 _index)))))
        (bind _result (Math|Integer|IncrementInt (.kol (.Value (Utilities|Map|Find (Variables|Default|GetStacks) (Utilities|Struct|MakeIntPoint _index_2 _index)))))
          (:%20%20
            (if (< (.kol (.Value (Utilities|Map|Find (Variables|Default|GetStacks) (Utilities|Struct|MakeIntPoint _index_2 _index)))) (Variables|/Game/Blueprints/Inventory/ItemData.ItemData_C|GetMax%20In%20Stack (.description (.Value (Utilities|Map|Find (Variables|Default|GetStacks) (Utilities|Struct|MakeIntPoint _index_2 _index))))))
              (Utilities|Map|Add (Variables|Default|GetStacks) (Utilities|Struct|MakeIntPoint _index_2 _index) (Utilities|Struct|MakeItemsStackStruct _result Description))
              (return true)))))))
  (for _index_3 (range 0 (- (.y _inventory_size) 1))
    (for _index_4 (range 0 (- (.x _inventory_size) 1))
      (if (.ReturnValue (Utilities|Map|Find (Variables|Default|GetStacks) (Utilities|Struct|MakeIntPoint _index_4 _index_3)))
        (if (== Description (.Description (Utilities|Struct|BreakItemsStackStruct (.Value (Utilities|Map|Find (Variables|Default|GetStacks) (Utilities|Struct|MakeIntPoint _index_4 _index_3))))))
          (if (< (.kol (.Value (Utilities|Map|Find (Variables|Default|GetStacks) (Utilities|Struct|MakeIntPoint _index_4 _index_3)))) (Variables|/Game/Blueprints/Inventory/ItemData.ItemData_C|GetMax%20In%20Stack Description))
            (bind _result_2 (Math|Integer|IncrementInt (.kol (.Value (Utilities|Map|Find (Variables|Default|GetStacks) (Utilities|Struct|MakeIntPoint _index_4 _index_3)))))
              (:%20%20
                (Utilities|Map|Add (Variables|Default|GetStacks) (Utilities|Struct|MakeIntPoint _index_4 _index_3) (Utilities|Struct|MakeItemsStackStruct _result_2 (.description (.Value (Utilities|Map|Find (Variables|Default|GetStacks) (Utilities|Struct|MakeIntPoint _index_4 _index_3))))))
                (return true)))))
        (else
          (Utilities|Map|Add (Variables|Default|GetStacks) (Utilities|Struct|MakeIntPoint _index_4 _index_3) (Utilities|Struct|MakeItemsStackStruct 1 Description))
          (return true)))))
  (return false))

(fn AddItems
  (params (Description :type Item%20Data%20Object%20Reference) (Kol%20Stack :type Integer))
  (for _index (range 0 (- Kol%20Stack 1))
    (bind _is_add_item (CallFunction|AddItem Description))
    (if _is_add_item
      (Math|Integer|IncrementInt (LocalVariables|GetAmout%20Add%20Item))))
  (return (LocalVariables|GetAmout%20Add%20Item)))

(fn DropItem
  (params (Position%20Drag%20item :type Int%20Point%20Structure) (Position%20Drop%20item :type Int%20Point%20Structure))
  (bind _stacks (Variables|Default|GetStacks))
  (bind _stacks_2 (Variables|Default|GetStacks))
  (bind (_value _returnvalue) (Utilities|Map|Find _stacks Position%20Drop%20item))
  (bind _value_2 (Utilities|Map|Find _stacks_2 Position%20Drag%20item))
  (bind (_kol _description) (Utilities|Struct|BreakItemsStackStruct _value_2))
  (bind (_kol_2 _description_2) (Utilities|Struct|BreakItemsStackStruct _value))
  (bind _returnvalue_2 (+ _kol _kol_2))
  (bind _max_in_stack (Variables|/Game/Blueprints/Inventory/ItemData.ItemData_C|GetMax%20In%20Stack _description_2))
  (bind _returnvalue_3 (Math|Integer|Clamp(Integer) _returnvalue_2 0 _max_in_stack))
  (bind _returnvalue_4 (- _returnvalue_2 _returnvalue_3))
  (if _returnvalue
    (if (!= Position%20Drag%20item Position%20Drop%20item)
      (if (== _description _description_2)
        (LocalVariables|SetDrop%20Amount _returnvalue_3)
        (LocalVariables|SetDrag%20Amount _returnvalue_4)
        (if (> _returnvalue_4 0)
          (Utilities|Map|Add (Variables|Default|GetStacks) Position%20Drag%20item (Utilities|Struct|MakeItemsStackStruct _returnvalue_4 _description))
          (else
            (Utilities|Map|Remove (Variables|Default|GetStacks) Position%20Drag%20item)))
        (Utilities|Map|Add (Variables|Default|GetStacks) Position%20Drop%20item (Utilities|Struct|MakeItemsStackStruct (LocalVariables|GetDrop%20Amount) _description_2))
        (CallFunction|UpdateUI)))
    (else
      ;[1 1 1] Move item
      (Utilities|Map|Add (Variables|Default|GetStacks) Position%20Drop%20item _value_2)
      (Utilities|Map|Remove (Variables|Default|GetStacks) Position%20Drag%20item)
      (CallFunction|UpdateUI))))

(fn RemoveItem
  (params (Description :type Item%20Data%20Object%20Reference))
  (bind _inventory_size (Variables|Default|GetInventory%20Size))
  (for _index (range 0 (- (.y _inventory_size) 1))
    (for _index_2 (range 0 (- (.x _inventory_size) 1))
      (LocalVariables|Setpos%20i (Utilities|Struct|MakeIntPoint _index_2 _index))
      (if (== Description (.description (.Value (Utilities|Map|Find (Variables|Default|GetStacks) (LocalVariables|Getpos%20i)))))
        (bind _result (Math|Integer|DecrementInt (.kol (.Value (Utilities|Map|Find (Variables|Default|GetStacks) (LocalVariables|Getpos%20i)))))
          (:%20%20
            (if (> _result 0)
              (Utilities|Map|Add (Variables|Default|GetStacks) (LocalVariables|Getpos%20i) (Utilities|Struct|MakeItemsStackStruct _result (.description (.Value (Utilities|Map|Find (Variables|Default|GetStacks) (LocalVariables|Getpos%20i))))))
              (else
                (Utilities|Map|Remove (Variables|Default|GetStacks) (LocalVariables|Getpos%20i))))
            (return true))))))
  (return false))

(fn RemoveItems
  (params (Description :type Item%20Data%20Object%20Reference) (Amount%20Stack :type Integer))
  (for _index (range 0 (- Amount%20Stack 1))
    (bind _is_add_item (CallFunction|RemoveItem Description))
    (if _is_add_item
      (Math|Integer|IncrementInt (LocalVariables|GetAmount%20Remove%20Item))))
  (bind _asplayer (Utilities|Casting|CastToPlayer (Game|Player|GetPlayerPawn 0)))
  (Utilities|IsValid (Variables|/Game/Blueprints/Player/Player.Player_C|GetUI%20Inventory _asplayer)
    (:Is%20Valid
      (Default|Update (Variables|/Game/Blueprints/Player/Player.Player_C|GetUI%20Inventory _asplayer))
      (return (LocalVariables|GetAmount%20Remove%20Item)))))

(fn RemoveCell
  (params (Remove%20pos :type Int%20Point%20Structure) (Amount :type Integer))
  (bind _stacks (Variables|Default|GetStacks))
  (bind _value (Utilities|Map|Find _stacks Remove%20pos))
  (bind _returnvalue (- (.kol _value) Amount))
  (if (!= Amount -1)
    (if (> _returnvalue 0)
      (Utilities|Map|Add (Variables|Default|GetStacks) Remove%20pos (Utilities|Struct|MakeItemsStackStruct _returnvalue (.description _value)))
      (else
        (Utilities|Map|Remove (Variables|Default|GetStacks) Remove%20pos :!label _label)))
    (else
      (goto _label)))
  (CallFunction|UpdateUI))

(fn SpawnItem
  (params (Item%20Drag :type Item%20Drag%20Object%20Reference))
  (bind _returnvalue (Game|Player|GetPlayerPawn 0))
  (bind _returnvalue_2 (Transformation|GetActorLocation _returnvalue))
  (bind _stack (Variables|/Game/Blueprints/Inventory/ItemDrag.ItemDrag_C|GetStack Item%20Drag))
  (bind (_kol _description) (Utilities|Struct|BreakItemsStackStruct _stack))
  (bind (_outhit _returnvalue_3) (Collision|SphereTraceByChannel _returnvalue_2 (+ _returnvalue_2 (* (Transformation|GetActorForwardVector _returnvalue) "200.000000,200.000000,0.000000")) 0.0 "TraceTypeQuery1" false 0 "None"))
  (if _returnvalue_3
    (LocalVariables|SetSpawn%20Location%20Start (- (.Location (Collision|BreakHitResult _outhit)) (* (Transformation|GetActorForwardVector (Game|Player|GetPlayerPawn 0)) "20.000000,20.000000,0.000000")))
    (LocalVariables|SetSpawn%20Location%20End (+ (- (.Location (Collision|BreakHitResult _outhit)) (* (Transformation|GetActorForwardVector (Game|Player|GetPlayerPawn 0)) "20.000000,20.000000,0.000000")) "0.000000,0.000000,-200.000000"))
    (else
      (LocalVariables|SetSpawn%20Location%20Start (.TraceEnd (Collision|BreakHitResult _outhit)))
      (LocalVariables|SetSpawn%20Location%20End (+ (.TraceEnd (Collision|BreakHitResult _outhit)) "0.000000,0.000000,-200.000000"))))
  (bind _outhit_2 (Collision|LineTraceByChannel (LocalVariables|GetSpawn%20Location%20Start) (LocalVariables|GetSpawn%20Location%20End) "TraceTypeQuery1" false 0 "None"))
  (Game|SpawnActorfromClass "/Game/Blueprints/InteractItem/Items_Def.Items_Def_C" (Math|Transform|MakeTransform (.Location (Collision|BreakHitResult _outhit_2)) "0, 0, 0" "1.000000,1.000000,1.000000") "Undefined" "MultiplyWithRoot" 0 _kol _description 0)
  (CallFunction|RemoveCell (Variables|/Game/Blueprints/Inventory/ItemDrag.ItemDrag_C|GetPosition Item%20Drag) (.Kol (Utilities|Struct|BreakItemsStackStruct (Variables|/Game/Blueprints/Inventory/ItemDrag.ItemDrag_C|GetStack Item%20Drag)))))

(fn UpdateUI
  (bind _asplayer (Utilities|Casting|CastToPlayer (Game|Player|GetPlayerPawn 0)))
  (Utilities|IsValid (Variables|/Game/Blueprints/Player/Player.Player_C|GetUI%20Inventory _asplayer)
    (:Is%20Valid
      (Default|Update (Variables|/Game/Blueprints/Player/Player.Player_C|GetUI%20Inventory _asplayer)))))