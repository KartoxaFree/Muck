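; Player character with Enhanced Input movement, melee attack, camera-based interaction and an inventory toggle.
; Tick derives the movement state to set walk speeds and box-traces from the camera for InteractInterface targets.
; HealthComponent handles hunger, stamina, hits and death, which shows a Death widget.
; The attack animates the held Pick procedurally through a Delay-driven loop instead of a Timeline; hotbar scroll, quick drop and item-mesh updates are inactive.
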(event OnDeath(Health_Component)
  ;[1 1 1] Death
  (CallFunction|Death))

(event Input|EnhancedActionEvents|EnhancedInputActionPlayerInput_Jump
  (params (ActionValue :type Boolean) (ElapsedSeconds :type Float%20%28double-precision%29) (TriggeredSeconds :type Float%20%28double-precision%29) (InputAction :type Input%20Action%20Object%20Reference :default "/Game/Blueprints/Player/Input/PlayerInput_Jump.PlayerInput_Jump"))
  ;[1 1 1] Jumping
  (:Started
    (Character|Jump)
    (Variables|IsBool|SetIs%20Jumping true))
  (:Completed
    (Character|StopJumping)
    (Variables|IsBool|SetIs%20Jumping false)))

(event Input|EnhancedActionEvents|EnhancedInputActionPlayerInput_Look
  (params (ActionValue :type Vector%202D%20Structure) (ElapsedSeconds :type Float%20%28double-precision%29) (TriggeredSeconds :type Float%20%28double-precision%29) (InputAction :type Input%20Action%20Object%20Reference :default "/Game/Blueprints/Player/Input/PlayerInput_Look.PlayerInput_Look"))
  (bind _camera_sensitivity (Variables|Specifications|GetCamera%20Sensitivity))
  (bind _returnvalue (* ActionValue _camera_sensitivity))
  (bind (_x _y) (Math|Vector2D|BreakVector2D _returnvalue))
  ;[1 1 1] Camera control
  (if (not (Variables|/Script/Engine.PlayerController|GetbShowMouseCursor (Game|GetPlayerController 0)))
    (Pawn|Input|AddControllerYawInput _x)
    (Pawn|Input|AddControllerPitchInput (* _y -1.0))))

(event Input|EnhancedActionEvents|EnhancedInputActionPlayerInput_Move
  (params (ActionValue :type Vector%202D%20Structure) (ElapsedSeconds :type Float%20%28double-precision%29) (TriggeredSeconds :type Float%20%28double-precision%29) (InputAction :type Input%20Action%20Object%20Reference :default "/Game/Blueprints/Player/Input/PlayerInput_Move.PlayerInput_Move"))
  (bind _returnvalue (Pawn|GetControlRotation :!class /Script/Engine.Pawn))
  ;[1 1 1] Movment
  (Pawn|Input|AddMovementInput (Math|Vector|GetRightVector (Math|Rotator|MakeRotator (.roll _returnvalue) 0.0 (.yaw _returnvalue))) (.x ActionValue) false)
  (Pawn|Input|AddMovementInput (Math|Vector|GetForwardVector (Math|Rotator|MakeRotator 0.0 0.0 (.yaw (Pawn|GetControlRotation :!class /Script/Engine.Pawn)))) (.y ActionValue) false))

(event Input|EnhancedActionEvents|EnhancedInputActionPlayerInput_E
  (params (ActionValue :type Boolean) (ElapsedSeconds :type Float%20%28double-precision%29) (TriggeredSeconds :type Float%20%28double-precision%29) (InputAction :type Input%20Action%20Object%20Reference :default "/Game/Blueprints/Player/Input/PlayerInput_E.PlayerInput_E"))
  ;[1 1 1] Interact
  (Class|InteractInterface|InteractE(Message) (Variables|Default|GetInteractable%20Actor) self (Variables|Default|GetInteractable%20Component)))

(event Input|EnhancedActionEvents|EnhancedInputActionPlayerInput_Crouch
  (params (ActionValue :type Boolean) (ElapsedSeconds :type Float%20%28double-precision%29) (TriggeredSeconds :type Float%20%28double-precision%29) (InputAction :type Input%20Action%20Object%20Reference :default "/Game/Blueprints/Player/Input/PlayerInput_Crouch.PlayerInput_Crouch"))
  ;[1 1 1] Crouching
  (:Triggered
    (Character|Crouch))
  (:Completed
    (Character|UnCrouch)))

(event Input|EnhancedActionEvents|EnhancedInputActionPlayerInput_Left_Click
  (params (ActionValue :type Boolean) (ElapsedSeconds :type Float%20%28double-precision%29) (TriggeredSeconds :type Float%20%28double-precision%29) (InputAction :type Input%20Action%20Object%20Reference :default "/Game/Blueprints/Player/Input/PlayerInput_Left_Click.PlayerInput_Left_Click"))
  (bind _returnvalue (Utilities|Time|GetWorldDeltaSeconds))
  (bind _returnvalue_2 (Utilities|Time|GetWorldDeltaSeconds))
  ;[1 1 1] Bonk
  (if (not (Variables|IsBool|GetIs%20Attack))
    (Variables|IsBool|SetIs%20Attack true)
    (Variables|Default|SetLocal%20Timeline 0.0)
    (bind _output_get (Variables|Default|SetLocal%20Timeline (+ (Variables|Default|GetLocal%20Timeline) (* _returnvalue_2 (Variables|Default|GetBonk%20Duration))) :!label _label))
    (if (<= _output_get 1.0)
      (if (<= (Variables|Default|GetLocal%20Timeline) 0.7)
        _
        (else
          (Default|HitActor (Variables|Default|GetHealth_Component) (Variables|Default|GetPickCollider))))
      (Utilities|FlowControl|Delay (/ _returnvalue_2 (Variables|Default|GetBonk%20Duration)))
      (Utilities|Bonk _output_get (Variables|Default|GetPick)
        (:End
          (goto _label)))
      (else
        (Default|EndHit (Variables|Default|GetHealth_Component))
        (Utilities|FlowControl|Delay 0.2)
        (Variables|Default|SetLocal%20Timeline 1.0)
        (bind _output_get_2 (Variables|Default|SetLocal%20Timeline (- (Variables|Default|GetLocal%20Timeline) (* _returnvalue (Variables|Default|GetBonk%20Duration))) :!label _label_2))
        (if (>= _output_get_2 0.0)
          (Utilities|FlowControl|Delay (/ _returnvalue (Variables|Default|GetBonk%20Duration)))
          (Utilities|Bonk _output_get_2 (Variables|Default|GetPick)
            (:End
              (goto _label_2)))
          (else
            (Variables|IsBool|SetIs%20Attack false)))))))

(event Input|EnhancedActionEvents|EnhancedInputActionPlayerInput_Sprint
  (params (ActionValue :type Boolean) (ElapsedSeconds :type Float%20%28double-precision%29) (TriggeredSeconds :type Float%20%28double-precision%29) (InputAction :type Input%20Action%20Object%20Reference :default "/Game/Blueprints/Player/Input/PlayerInput_Sprint.PlayerInput_Sprint"))
  ;[1 1 1] Sprint
  (:Triggered
    (Variables|IsBool|SetIs%20Sprinting (> (Variables|/Game/Blueprints/Health/Health_Component.Health_Component_C|GetStamina%20Actor (Variables|Default|GetHealth_Component)) 0.0)))
  (:Started
    (Variables|IsBool|SetIs%20Sprinting true)
    (Variables|/Game/Blueprints/Health/Health_Component.Health_Component_C|Setis%20Sprinting (Variables|Default|GetHealth_Component) (Variables|IsBool|GetIs%20Sprinting) :!label _label))
  (:Completed
    (Variables|IsBool|SetIs%20Sprinting false)
    (goto _label)))

(event Input|EnhancedActionEvents|EnhancedInputActionPlayerInput_Inventory
  (params (ActionValue :type Boolean) (ElapsedSeconds :type Float%20%28double-precision%29) (TriggeredSeconds :type Float%20%28double-precision%29) (InputAction :type Input%20Action%20Object%20Reference :default "/Game/Blueprints/Player/Input/PlayerInput_Inventory.PlayerInput_Inventory"))
  (bind _inventory_full (Variables|Default|GetInventory_Full))
  (bind _ui_inventory (Variables|/Game/Blueprints/Inventory/Inventory_Component.Inventory_component_C|GetUI%20Inventory _inventory_full))
  ;[1 1 1] Create Inventory
  (Utilities|IsValid _ui_inventory
    (:Is%20Valid
      (CallFunction|BlockMouse false _ui_inventory)
      (Default|DeleteInventory (Variables|Default|GetInventory_Full)))
    (:Is%20Not%20Valid
      (CallFunction|BlockMouse true _ui_inventory)
      (Default|CreateUIInventory (Variables|Default|GetInventory_Full) (Utilities|Struct|MakeIntPoint 11 5)))))

(event Input|EnhancedActionEvents|EnhancedInputActionPlayerInput_Scroll
  (params (ActionValue :type Float%20%28double-precision%29) (ElapsedSeconds :type Float%20%28double-precision%29) (TriggeredSeconds :type Float%20%28double-precision%29) (InputAction :type Input%20Action%20Object%20Reference :default "/Game/Blueprints/Player/Input/PlayerInput_Scroll.PlayerInput_Scroll"))
  ;[1 1 1] Scroll hot bar
)

(event Input|EnhancedActionEvents|EnhancedInputActionPlayerInput_Drop_Item
  (params (ActionValue :type Boolean) (ElapsedSeconds :type Float%20%28double-precision%29) (TriggeredSeconds :type Float%20%28double-precision%29) (InputAction :type Input%20Action%20Object%20Reference :default "/Game/Blueprints/Player/Input/PlayerInput_Drop_Item.PlayerInput_Drop_Item"))
  ;[1 1 1] Fast Drop q
)

(event EventBeginPlay
  (bind _asplayer_controller (Utilities|Casting|CastToPlayerController (Pawn|GetController)))
  (Utilities|IsValid (PlayerController|LocalPlayerSubsystems|GetEnhancedInputLocalPlayerSubsystem _asplayer_controller)
    (:Is%20Valid
      (Input|AddMappingContext (PlayerController|LocalPlayerSubsystems|GetEnhancedInputLocalPlayerSubsystem _asplayer_controller) "/Game/Blueprints/Player/Input/Custom.Custom" 0 "(bIgnoreAllPressedKeysUntilRelease=True,bForceImmediately=False,bNotifyUserSettings=False)")
      ;[1 1 1] UI Interaction
      (bind _returnvalue (UserInterface|CreateWidget "/Game/UI/Interaction.Interaction_C"))
      (bind _output_get (Variables|UI|SetUI%20Interaction _returnvalue))
      (UserInterface|Viewport|AddtoViewport _output_get 0)
      (Variables|/Game/Blueprints/Health/Health_Component.Health_Component_C|SetHealth%20Actor (Variables|Default|GetHealth_Component) 1e+02)
      (Variables|/Game/Blueprints/Health/Health_Component.Health_Component_C|SetDamage%20Actor (Variables|Default|GetHealth_Component) (Variables|Specifications|GetBase%20Damage))
      (Default|CreateUI (Variables|Default|GetHealth_Component))
      (Variables|/Game/Blueprints/Health/Health_Component.Health_Component_C|SetisHunger (Variables|Default|GetHealth_Component) true)
      (Default|HungerUpdate (Variables|Default|GetHealth_Component)))))

(event EventTick
  (params (DeltaSeconds :type Float%20%28single-precision%29))
  (CallFunction|MovmentState)
  (|Interaction 3e+02)
  (CallFunction|SetMeshItem))

(fn ConstructionScript)

(fn MovmentState
  (Utilities|FlowControl|Sequence
    (:then_0
      (if (== (Math|Vector|VectorLength (Transformation|GetVelocity)) 0.0)
        (LocalVariables|SetNew%20State%20Moving "NewEnumerator0")
        (elif (AI|Components|NavMovement|IsMovingonGround (Variables|Character|GetCharacterMovement))
          (if (AI|Components|NavMovement|IsCrouching (Variables|Character|GetCharacterMovement))
            (LocalVariables|SetNew%20State%20Moving "NewEnumerator3")
            (elif (Variables|IsBool|GetIs%20Sprinting)
              (LocalVariables|SetNew%20State%20Moving "NewEnumerator2")
              (else
                (LocalVariables|SetNew%20State%20Moving "NewEnumerator1"))))
          (else
            (LocalVariables|SetNew%20State%20Moving "NewEnumerator4")))))
    (:then_1
      (if (Utilities|Enum|NotEqual(Enum) (Variables|Default|GetState%20Moving) (LocalVariables|GetNew%20State%20Moving))
        (Variables|Default|SetState%20Moving (LocalVariables|GetNew%20State%20Moving))
        (CallFunction|SetSpeed)))))

(fn OnRepCurrentState)

(fn SetSpeed
  (bind _charactermovement (Variables|Character|GetCharacterMovement))
  (switch Utilities|FlowControl|Switch|SwitchonMovementStateEnum (Variables|Default|GetState%20Moving)
    (:NewEnumerator1
      (Variables|/Script/Engine.CharacterMovementComponent|SetMaxWalkSpeed _charactermovement (LocalVariables|GetWalk%20Speed)))
    (:NewEnumerator2
      (Variables|/Script/Engine.CharacterMovementComponent|SetMaxWalkSpeed _charactermovement (LocalVariables|GetSprint%20Speed)))
    (:NewEnumerator3
      (Variables|/Script/Engine.CharacterMovementComponent|SetMaxWalkSpeedCrouched _charactermovement (LocalVariables|GetCroch%20Speed)))))

(fn Death
  (Development|PrintString "Death")
  (bind _returnvalue (UserInterface|CreateWidget "/Game/TestLocation/death.death_C"))
  (UserInterface|Viewport|AddtoViewport _returnvalue 0))

(fn SetMeshItem)

(fn BlockMouse
  (params (Add :type Boolean) (Name%20Param :type Widget%20Object%20Reference))
  (bind _returnvalue (Game|GetPlayerController 0))
  (bind _returnvalue_2 (Game|GetPlayerController 0))
  (if Add
    (Utilities|Array|Add (LocalVariables|GetAr%20Block%20Contorll) Name%20Param)
    (Variables|/Script/Engine.PlayerController|SetbShowMouseCursor _returnvalue_2 true)
    (Input|SetInputModeGameandUI _returnvalue_2 0 "DoNotLock" false false)
    (else
      (Utilities|Array|RemoveItem (LocalVariables|GetAr%20Block%20Contorll) Name%20Param)
      (if (Utilities|Array|IsEmpty (LocalVariables|GetAr%20Block%20Contorll))
        (Variables|/Script/Engine.PlayerController|SetbShowMouseCursor _returnvalue false)
        (Input|SetInputModeGameOnly _returnvalue false)))))

(fn SetProgressBar)