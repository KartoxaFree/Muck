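; Base pickup item actor that moves its stack into the interactor's inventory when interacted with.
; BeginPlay sets the Sphere mesh from the item Description's drop mesh.
; InteractE passes the description and stack count to the interactor's Inventory_Component and subtracts the amount added.
; The actor destroys itself when the stack is empty, otherwise a short delay gates the next interaction.
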(event EventBeginPlay
  (Components|StaticMesh|SetStaticMesh (Variables|Default|GetSphere) (Variables|/Game/Blueprints/Inventory/ItemData.ItemData_C|GetActor%20Drop (Variables|Default|GetDescription))))

(event EventInteractE
  (params (Interactor :type Player%20Object%20Reference) (HitComponent :type Primitive%20Component%20Object%20Reference))
  (if (not (Variables|Default|GetDelay%20Interact))
    (Variables|Default|SetDelay%20Interact true)
    (bind _amount_add (Default|AddItems (Actor|GetComponentbyClass Interactor "/Game/Blueprints/Inventory/Inventory_Component.Inventory_Component_C") (Variables|Default|GetDescription) (Variables|Default|GetKol%20in%20Stack)))
    (bind _output_get (Variables|Default|SetKol%20in%20Stack (- (Variables|Default|GetKol%20in%20Stack) _amount_add)))
    (if (<= _output_get 0)
      (Actor|DestroyActor)
      (else
        (Utilities|FlowControl|Delay 0.5)
        (Variables|Default|SetDelay%20Interact false)))))

(fn ConstructionScript)