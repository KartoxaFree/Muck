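; Base actor for interactable dropped items, holding an item description and a stack count.
; The construction script sets the Sphere mesh from the description's drop mesh.
; InteractE only sets a delay flag to block repeat interaction, with no pickup call wired after it.
; AddItems reduces the stack, then destroys the actor when empty or clears the flag after a short delay.
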(event EventBeginPlay)

(event EventInteractE
  (params (Interactor :type Player%20Object%20Reference) (HitComponent :type Primitive%20Component%20Object%20Reference))
  (if (not (Variables|Default|GetDelay%20Interact))
    (Variables|Default|SetDelay%20Interact true)))

(fn ConstructionScript
  (Components|StaticMesh|SetStaticMesh (Variables|Default|GetSphere) (Variables|/Game/Blueprints/InteractItem/Items/ItemData.ItemData_C|GetActor%20Drop (Variables|Default|GetDescription))))